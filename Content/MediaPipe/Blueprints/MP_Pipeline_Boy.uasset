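; MediaPipe pipeline actor that recognizes three hand gestures and prints Korean bargaining phrases for them as debug text.
; Wrapper functions configure, start and stop the Pipeline component, whose video texture can display on a Cube through a dynamic material.
; DrawLandmarks draws an observer's detections and calls SetGesture, which tests gestures in priority order.
; Each gesture is a hard-coded chain of landmark axis comparisons, each gated by the previous result.
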(event OnVideoTextureCreated(Pipeline)
  (params (NewTexture :type Texture%202D%20Object%20Reference))
  (bind _cube (Variables|Default|GetCube))
  (if (Variables|Pipeline|GetEnableVideoTexture)
    (bind _returnvalue (Rendering|Material|CreateDynamicMaterialInstance "/Game/MediaPipe/Blueprints/MAT_VideoTexture.MAT_VideoTexture" "None" "Transient" :!class /Script/Engine.KismetMaterialLibrary))
    (Rendering|Material|SetTextureParameterValue _returnvalue "Video" NewTexture)
    (Rendering|Material|SetMaterial _cube 0 _returnvalue)
    (Rendering|SetVisibility _cube true false)))

(event EventBeginPlay)

(event EventTick
  (params (DeltaSeconds :type Float%20%28single-precision%29)))

(event EventEndPlay
  (params (EndPlayReason :type EEndPlayReason%20Enum :default "Destroyed")))

(fn ConstructionScript)

(fn StartPipeline
  (bind _pipeline (Variables|Default|GetPipeline))
  (if (Variables|Pipeline|GetEnableAutoStart)
    (Variables|/Script/MediaPipe.MediaPipePipelineComponent|SetInputFile _pipeline (Variables|Pipeline|GetInputFile))
    (Variables|/Script/MediaPipe.MediaPipePipelineComponent|SetCameraId _pipeline (Variables|Pipeline|GetCamId))
    (Variables|/Script/MediaPipe.MediaPipePipelineComponent|SetCaptureApi _pipeline (Variables|Pipeline|GetCaptureApi))
    (Variables|/Script/MediaPipe.MediaPipePipelineComponent|SetResX _pipeline (Variables|Pipeline|GetResX))
    (Variables|/Script/MediaPipe.MediaPipePipelineComponent|SetResY _pipeline (Variables|Pipeline|GetResY))
    (Variables|/Script/MediaPipe.MediaPipePipelineComponent|SetbEnableOverlay _pipeline (Variables|Pipeline|GetEnableOverlay))
    (Variables|/Script/MediaPipe.MediaPipePipelineComponent|SetbEnableVideoTexture _pipeline (Variables|Pipeline|GetEnableVideoTexture))
    (CameraShake|Start _pipeline)))

(fn StopPipeline
  (Audio|Components|Audio|Stop (Variables|Default|GetPipeline)))

(fn SetGraphNode
  (params (Node :type String))
  (Variables|/Script/MediaPipe.MediaPipePipelineComponent|SetGraphNodes (Variables|Default|GetPipeline) (Utilities|Array|MakeArray Node)))

(fn SetGraphNodes
  (params (Nodes :type Array%20of%20Strings))
  (Variables|/Script/MediaPipe.MediaPipePipelineComponent|SetGraphNodes (Variables|Default|GetPipeline) Nodes))

(fn DrawCameraOrigin
  (bind _cameraorigin (Variables|Pipeline|GetCameraOrigin))
  (Class|KismetSystemLibrary|DrawDebugCoordinateSystem _cameraorigin "0, 0, 0" 1e+01 0.0 0.0)
  (Rendering|Debug|DrawDebugBox :Center (+ _cameraorigin "0,50.000000,-50.000000") :Extent "5.000000,50.000000,50.000000"))

(fn DrawWorldOrigin
  (bind _worldorigin (Variables|Pipeline|GetWorldOrigin))
  (Class|KismetSystemLibrary|DrawDebugCoordinateSystem _worldorigin "0, 0, 0" 1e+01 0.0 0.0)
  (Rendering|Debug|DrawDebugBox _worldorigin "100.000000,100.000000,100.000000" "(R=0.000000,G=0.000000,B=0.000000,A=1.000000)" "0, 0, 0" 0.0 0.0))

(fn DrawLandmarks
  (params (Observer :type Media%20Pipe%20Landmark%20Observer%20Component%20Object%20Reference) (ObjectId :type Integer) (Origin :type Vector) (PrimitiveScale :type Float%20%28single-precision%29) (PrimitiveColor :type Linear%20Color%20Structure))
  (Utilities|IsValid Observer
    (:Is%20Valid
      (if (Class|MediaPipeObserverComponent|HaveDetections Observer)
        (Class|MediaPipeLandmarkObserverComponent|DrawDebugLandmarks Observer ObjectId (Math|Transform|MakeTransform Origin "0, 0, 0" "1,1,1") PrimitiveScale PrimitiveColor)
        (CallFunction|SetGesture Observer ObjectId)
        (Rendering|Debug|DrawDebugBox (+ Origin "0, 0, 0") "1.000000,1.000000,1.000000" PrimitiveColor "0, 0, 0" 0.0 0.0)))))

(fn CompareY
  (params (Idx1 :type Integer) (Idx2 :type Integer) (Observer :type Media%20Pipe%20Landmark%20Observer%20Component%20Object%20Reference) (ObjectID :type Integer) (Check :type Boolean))
  (if Check
    (Math|Float|CompareFloat (.Y (Math|Vector|BreakVector (.Pos (Utilities|Struct|BreakMediaPipeLandmark (Class|MediaPipeLandmarkObserverComponent|GetLandmark Observer ObjectID Idx1))))) (.Y (Math|Vector|BreakVector (.Pos (Utilities|Struct|BreakMediaPipeLandmark (Class|MediaPipeLandmarkObserverComponent|GetLandmark Observer ObjectID Idx2)))))
      (:>
        (return true))
      (:==
        _)
      (:<
        _)))
  (return false))

(fn CompareX
  (params (Idx1 :type Integer) (Idx2 :type Integer) (Observer :type Media%20Pipe%20Landmark%20Observer%20Component%20Object%20Reference) (ObjectID :type Integer) (Check :type Boolean))
  (if Check
    (Math|Float|CompareFloat (.X (Math|Vector|BreakVector (.Pos (Utilities|Struct|BreakMediaPipeLandmark (Class|MediaPipeLandmarkObserverComponent|GetLandmark Observer ObjectID Idx1))))) (.X (Math|Vector|BreakVector (.Pos (Utilities|Struct|BreakMediaPipeLandmark (Class|MediaPipeLandmarkObserverComponent|GetLandmark Observer ObjectID Idx2)))))
      (:>
        (return true))
      (:==
        _)
      (:<
        _)))
  (return false))

(fn CompareZ
  (params (Idx1 :type Integer) (Idx2 :type Integer) (Observer :type Media%20Pipe%20Landmark%20Observer%20Component%20Object%20Reference) (ObjectID :type Integer) (Check :type Boolean))
  (if Check
    (Math|Float|CompareFloat (.Z (Math|Vector|BreakVector (.Pos (Utilities|Struct|BreakMediaPipeLandmark (Class|MediaPipeLandmarkObserverComponent|GetLandmark Observer ObjectID Idx1))))) (.Z (Math|Vector|BreakVector (.Pos (Utilities|Struct|BreakMediaPipeLandmark (Class|MediaPipeLandmarkObserverComponent|GetLandmark Observer ObjectID Idx2)))))
      (:>
        (return true))
      (:==
        _)
      (:<
        _)))
  (return false))

(fn Gesture1
  (params (Observer :type Media%20Pipe%20Landmark%20Observer%20Component%20Object%20Reference) (Object%20ID :type Integer))
  (bind _rcheck (CallFunction|CompareY 5 4 Observer Object%20ID (Variables|Default|Getcheck)))
  (bind _rcheck_2 (CallFunction|CompareZ 8 6 Observer Object%20ID _rcheck))
  (bind _rcheck_3 (CallFunction|CompareZ 12 10 Observer Object%20ID _rcheck_2))
  (bind _rcheck_4 (CallFunction|CompareZ 16 14 Observer Object%20ID _rcheck_3))
  (bind _rcheck_5 (CallFunction|CompareZ 20 18 Observer Object%20ID _rcheck_4))
  (bind _rcheck_6 (CallFunction|CompareZ 4 2 Observer Object%20ID _rcheck_5))
  (return _rcheck_6))

(fn Gesture2
  (params (Observer :type Media%20Pipe%20Landmark%20Observer%20Component%20Object%20Reference) (Object%20ID :type Integer))
  (bind _rcheck (CallFunction|CompareY 20 18 Observer Object%20ID (Variables|Default|Getcheck)))
  (bind _rcheck_2 (CallFunction|CompareY 16 14 Observer Object%20ID _rcheck))
  (bind _rcheck_3 (CallFunction|CompareY 12 10 Observer Object%20ID _rcheck_2))
  (bind _rcheck_4 (CallFunction|CompareY 8 6 Observer Object%20ID _rcheck_3))
  (bind _rcheck_5 (CallFunction|CompareZ 2 4 Observer Object%20ID _rcheck_4))
  (return _rcheck_5))

(fn Gesture3
  (params (Observer :type Media%20Pipe%20Landmark%20Observer%20Component%20Object%20Reference) (Object%20ID :type Integer))
  (bind _rcheck (CallFunction|CompareY 5 4 Observer Object%20ID (Variables|Default|Getcheck)))
  (bind _rcheck_2 (CallFunction|CompareZ 4 2 Observer Object%20ID _rcheck))
  (bind _rcheck_3 (CallFunction|CompareZ 8 6 Observer Object%20ID _rcheck_2))
  (bind _rcheck_4 (CallFunction|CompareZ 10 12 Observer Object%20ID _rcheck_3))
  (bind _rcheck_5 (CallFunction|CompareZ 14 16 Observer Object%20ID _rcheck_4))
  (bind _rcheck_6 (CallFunction|CompareZ 18 20 Observer Object%20ID _rcheck_5))
  (return _rcheck_6))

(fn SetGesture
  (params (Observer :type Media%20Pipe%20Landmark%20Observer%20Component%20Object%20Reference) (ObjectID :type Integer))
  (bind _rcheck (CallFunction|Gesture1 Observer ObjectID))
  (if _rcheck
    (Development|PrintString "안됩니다!" true false "(R=0.000000,G=0.660000,B=1.000000,A=1.000000)" 0.0)
    (else
      (bind _rcheck_2 (CallFunction|Gesture2 Observer ObjectID))
      (if _rcheck_2
        (Development|PrintString "가격을 깎아주세요" true false "(R=0.000000,G=0.660000,B=1.000000,A=1.000000)" 0.0)
        (else
          (bind _rcheck_3 (CallFunction|Gesture3 Observer ObjectID))
          (if _rcheck_3
            (Development|PrintString "서비스로 조금만 더 주세요" true false "(R=0.000000,G=0.660000,B=1.000000,A=1.000000)" 0.0)))))))